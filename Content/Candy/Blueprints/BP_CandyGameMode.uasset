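; BP_CandyGameMode is the game mode for the candy multiplayer game, tracking each player's name, index and score.
; On PostLogin it registers the controller, assigns a sequential index and default name to controller and PlayerState, and zeroes the score.
; Score additions update both the shared list and the controller, then RefreshUI sends name and score lists to every controller.
; An authority-only event teleports players' pawns to supplied locations by index.
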(event Custom|RefreshUI
  (for _array_element (Variables|Default|GetPlayerControllerList)
    (Default|InitUI _array_element (Variables|Default|GetNameList) (Variables|Default|GetScoreList))))

(event Custom|AddPlayerScore
  (params (PlayerIndex :type Integer) (Score :type Integer))
  (bind _playercontrollerlist (Variables|Default|GetPlayerControllerList))
  (bind _scorelist (Variables|Default|GetScoreList))
  (bind _output (Utilities|Array|Get(acopy) _playercontrollerlist PlayerIndex))
  (Utilities|Array|SetArrayElem _scorelist PlayerIndex (+ (Utilities|Array|Get(acopy) _scorelist PlayerIndex) Score))
  (Variables|/Game/Candy/Blueprints/BP_CandyPlayerController.BP_CandyPlayerController_C|SetScore _output (+ (Variables|/Game/Candy/Blueprints/BP_CandyPlayerController.BP_CandyPlayerController_C|GetScore _output) Score))
  (CallFunction|RefreshUI))

(event Custom|ResetPlayerLocation
  (params (LocationList :type Array%20of%20Vectors))
  (Networking|SwitchHasAuthority
    (:Authority
      (for (_array_element _array_index) (Variables|Default|GetPlayerControllerList)
        (Transformation|SetActorLocation (Pawn|GetControlledPawn _array_element) (Utilities|Array|Get(acopy) LocationList _array_index) false false)))))

(event EventTick
  (params (DeltaSeconds :type Float%20%28single-precision%29)))

(event EventPostLogin
  (params (NewPlayer :type Player%20Controller%20Object%20Reference))
  (bind _currentindex (Variables|Default|GetCurrentIndex))
  (bind _returnvalue (Utilities|String|ToString(Integer) _currentindex))
  (bind _returnvalue_2 (Utilities|String|Append "Player" _returnvalue))
  (bind _asbp_candy_player_controller (Utilities|Casting|CastToBP_CandyPlayerController NewPlayer))
  (Utilities|Array|Add (Variables|Default|GetPlayerControllerList) _asbp_candy_player_controller)
  (Utilities|Array|Add (Variables|Default|GetNameList) _returnvalue_2)
  (Variables|/Game/Candy/Blueprints/BP_CandyPlayerController.BP_CandyPlayerController_C|SetName _asbp_candy_player_controller _returnvalue_2)
  (Variables|/Game/Candy/Blueprints/BP_CandyPlayerController.BP_CandyPlayerController_C|SetPlayerIndex _asbp_candy_player_controller _currentindex)
  (Variables|/Game/Candy/Blueprints/BP_CandyPlayerController.BP_CandyPlayerController_C|SetScore _asbp_candy_player_controller 0)
  (bind _asbp_player_state (Utilities|Casting|CastToBP_PlayerState (Variables|/Script/Engine.Controller|GetPlayerState _asbp_candy_player_controller)))
  (Variables|/Game/Candy/Blueprints/BP_PlayerState.BP_PlayerState_C|SetPlayerIndex _asbp_player_state _currentindex)
  (Utilities|Array|Add (Variables|Default|GetScoreList) 0)
  (Math|Integer|IncrementInt (Variables|Default|GetCurrentIndex)
    (:%20%20
      (CallFunction|RefreshUI))))

(fn ConstructionScript)